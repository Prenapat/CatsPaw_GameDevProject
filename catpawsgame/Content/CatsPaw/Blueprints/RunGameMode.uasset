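; Game mode for a runner that builds a procedural track and shows the RunHUD widget at BeginPlay.
; It seeds the track with ten AddFloorTile calls, spawning random straight tiles and switching to a random curve once the straight counter exceeds its limit, then resetting it.
; Each spawned BP_FloorTile returns an attach transform that becomes the next spawn point, chaining the pieces end to end.
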(event `self.ReceiveBeginPlay`
  (bind _returnvalue (`|CreateWidget` "/Game/CatsPaw/UMG/RunHUD.RunHUD_C"))
  (`UserWidget.AddToViewport` _returnvalue 0)
  (for _ (range 10)
    (`self.AddFloorTile`)))

(fn `AddFloorCurve`
  (bind _floorcurves (`self.FloorCurves`))
  (bind _returnvalue (`|SpawnActorFromClass` (`|GetArrayItem` _floorcurves (`KismetMathLibrary.RandomIntegerInRange` 0 (`KismetArrayLibrary.Array_LastIndex` _floorcurves))) (`self.NextSpawnPoint`) "Undefined" "OverrideRootScale" null null))
  (bind _asbp_floor_tile (cast `/Game/CatsPaw/Blueprints/BP_FloorTile` _returnvalue))
  (bind _attachtranform (`/Game/CatsPaw/Blueprints/BP_FloorTile.GetAttachTransform` _asbp_floor_tile))
  (set `self.NextSpawnPoint` _attachtranform)
  (set `self.CurrentStraights` 0))

(fn `AddFloorTile`
  (bind _floortiles (`self.FloorTiles`))
  (if (> (`self.CurrentStraights`) 7)
    (`self.AddFloorCurve`)
    (else
      (bind _returnvalue (`|SpawnActorFromClass` (`|GetArrayItem` _floortiles (`KismetMathLibrary.RandomIntegerInRange` 0 (`KismetArrayLibrary.Array_LastIndex` _floortiles))) (`self.NextSpawnPoint`) "Undefined" "OverrideRootScale" null null))
      (bind _asbp_floor_tile (cast `/Game/CatsPaw/Blueprints/BP_FloorTile` _returnvalue))
      (bind _attachtranform (`/Game/CatsPaw/Blueprints/BP_FloorTile.GetAttachTransform` _asbp_floor_tile))
      (set `self.NextSpawnPoint` _attachtranform)
      (set `self.CurrentStraights` (+ (`self.CurrentStraights`) 1)))))

(fn `UserConstructionScript`)